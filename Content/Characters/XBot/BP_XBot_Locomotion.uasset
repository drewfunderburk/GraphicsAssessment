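; XBot character Blueprint that turns player axis input into camera-relative movement and controller look, with optional inverted pitch.
; Move inputs follow the camera's forward and right vectors, flattened to the horizontal plane and normalized.
; After each move input, it converts velocity to actor-local space, divides X and Y by max speed, and writes the result to the AnimBP's AnimVelocity to inform animation.
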(event EventBeginPlay
  (|CallParentFunction) ; This node is disabled and will not be called.\nDrag off pins to build functionality.
)

(event Input|AxisEvents|InputAxisMoveForward
  (params (AxisValue :type Float%20%28single-precision%29))
  ;[1 1 1] Movement
  (|MoveForward AxisValue (.Forward (|GetCameraVectorsNormalized)))
  (|SetAnimVelocity))

(event Input|AxisEvents|InputAxisMoveRight
  (params (AxisValue :type Float%20%28single-precision%29))
  ;[1 1 1] Movement
  (|MoveRight AxisValue (.Right (|GetCameraVectorsNormalized)))
  (|SetAnimVelocity))

(event Input|AxisEvents|InputAxisAimX
  (params (AxisValue :type Float%20%28single-precision%29))
  ;[1 1 1] Aim
  (Pawn|Input|AddControllerYawInput AxisValue))

(event Input|AxisEvents|InputAxisAimY
  (params (AxisValue :type Float%20%28single-precision%29))
  ;[1 1 1] Aim
  (if (Variables|Default|GetInvertY)
    (Pawn|Input|AddControllerPitchInput (* AxisValue -1.0))
    (else
      (Pawn|Input|AddControllerPitchInput AxisValue))))

(fn ConstructionScript
  (|CallParentFunction))