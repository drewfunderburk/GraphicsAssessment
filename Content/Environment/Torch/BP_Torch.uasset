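; BP_Torch is an environment torch whose point light flickers.
; BeginPlay stores the light's starting intensity and picks a random noise time offset, so each torch starts at its own phase.
; Each Tick samples 1D Perlin noise, remaps it to scale intensity between half and full of the starting value, then advances the noise time by PulseRate times world delta seconds.
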(event EventTick
  (params (DeltaSeconds :type Float%20%28single-precision%29))
  (Rendering|Components|Light|SetIntensity (Variables|Default|GetPointLight) (* (Variables|Light|GetPointLightStartValue) (/ (+ (/ (+ (Class|KismetMathLibrary|PerlinNoise1D (Variables|Light|GetCurrentPulseTime)) 1.0) 2.0) 1.0) 2.0)))
  (Variables|Light|SetCurrentPulseTime (+ (* (Variables|Light|GetPulseRate) (Utilities|Time|GetWorldDeltaSeconds)) (Variables|Light|GetCurrentPulseTime))))

(event EventBeginPlay
  (Variables|Light|SetPointLightStartValue (Variables|/Script/Engine.LightComponentBase|GetIntensity (Variables|Default|GetPointLight)))
  (Variables|Light|SetCurrentPulseTime (* (Math|Random|RandomFloat) 5e+03)))

(fn ConstructionScript)